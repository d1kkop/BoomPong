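; BallShooter is an actor that fires BallBP balls on a left mouse click while moving along a looping path.
; Each click spawns a ball at the shooter's transform and gives it a random force along X, with zero spin.
; Tick accumulates time and offsets the shooter from its BeginPlay location using sine and cosine, tracing a scalable figure eight in the YZ plane.
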(event `Key|LeftMouseButton`
  (params (Key :type "Key Structure" :default "AnyKey"))
  (:`Pressed`
    (bind _returnvalue (`|SpawnActorFromClass` "/Game/Blueprints/BallBP.BallBP_C" (`self.GetTransform`) "AlwaysSpawn" "OverrideRootScale"))
    (`Ball.AddForce` _returnvalue (`KismetMathLibrary.MakeVector` (`KismetMathLibrary.RandomFloatInRange` 400.0 600.0)))
    (`Ball.AddSpin` _returnvalue (`KismetMathLibrary.MakeVector` 0.0 0.0))))

(event `self.ReceiveBeginPlay`
  (set `self.Original` (`self.K2_GetActorLocation`)))

(event `self.ReceiveTick`
  (params (DeltaSeconds :type "Float (single-precision)"))
  (bind _scale (`self.Scale`))
  (bind _output_get (set `self.Time` (+ DeltaSeconds (`self.Time`))))
  (`self.K2_SetActorLocation` (+ (`KismetMathLibrary.MakeVector` 0.0 (* (`KismetMathLibrary.Cos` (+ _output_get (* (`KismetMathLibrary.GetPI`) 0.5))) _scale) (* (`KismetMathLibrary.Sin` (* _output_get 2.0)) _scale (`self.HeightScale`))) (`self.Original`))))

(fn `UserConstructionScript`)