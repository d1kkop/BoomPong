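; SplineFollower is an actor that records and replays behaviour on key presses and activates its own camera at BeginPlay.
; K starts the Recorder; later presses stop it and save "Recorded_Behaviour", since WasRecording is never cleared.
; L loads that saved record into RecordPlayer and plays it.
; Despite the name, the graphs contain no spline-following logic.
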(event `Key|K`
  (params (Key :type "Key Structure" :default "AnyKey"))
  (bind _recorder (`self.Recorder`))
  (:`Pressed`
    (if (`self.WasRecording`)
      (`Recorder.StopRecord` _recorder)
      (`Recorder.SaveRecord` _recorder "Recorded_Behaviour")
      (else
        (`Recorder.StartRecord` _recorder)
        (set `self.WasRecording` true)))))

(event `Key|L`
  (params (Key :type "Key Structure" :default "AnyKey"))
  (bind _recordplayer (`self.RecordPlayer`))
  (:`Pressed`
    (`RecordPlayer.Load` _recordplayer "Recorded_Behaviour")
    (`RecordPlayer.Play` _recordplayer -1.0)))

(event `self.ReceiveBeginPlay`
  (`ActorComponent.Activate` (`self.Camera`) false)
  (`ActorComponent.SetActive` (`self.Camera`) true false))

(fn `UserConstructionScript`)